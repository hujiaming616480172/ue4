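; Weapon Blueprint that provides automatic fire by spawning Zidan actors at the Zidanspawn component's world transform.
; Pulling the trigger passes a DoOnce gate, fires immediately, then starts a looping timer that repeats the fire event at an interval derived from FirePerSecond.
; Releasing the trigger clears the timer and resets the gate for the next pull.
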(event Custom|pulltriggle\
  (Utilities|FlowControl|DoOnce false
    (:Completed
      (CallFunction|Fire)
      (Utilities|Time|SetTimerbyFunctionName 0 "fire" (/ 1.0 (Variables|Default|Getfire%20per%20second)) true))))

(event Custom|fire
  (Game|SpawnActorfromClass "/Game/blueprints/zidan.zidan_C" (Transformation|GetWorldTransform (Variables|Default|Getzidanspawn)) "Undefined" 0 0))

(event Custom|release
  (Utilities|Time|ClearTimerbyFunctionName 0 "fire")
  (Utilities|FlowControl|DoOnce false) ; enters at Reset
)

(event EventBeginPlay)

(event Collision|EventActorBeginOverlap
  (params (OtherActor :type Actor%20Object%20Reference)))

(event EventTick
  (params (DeltaSeconds :type Float%20%28single-precision%29)))

(fn ConstructionScript)