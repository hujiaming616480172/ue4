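; A HUD Blueprint that creates the game's start menu, health display and pause menu widgets.
; On BeginPlay it shows the cursor, opens the Start widget with UI-only input and pauses the game, then adds the Basecharacterhealth widget to the viewport.
; The pressH event opens a new Pause widget the same way, with cursor, UI-only input and a paused game.
; Nothing here resumes play or removes the widgets.
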(event Custom|press%20H
  (Variables|/Script/Engine.PlayerController|SetbShowMouseCursor (Game|GetPlayerController 0) true)
  (bind _returnvalue (UserInterface|CreateWidget "/Game/blueprints/pause.pause_C"))
  (bind _output_get (Variables|Default|Setpause _returnvalue))
  (Input|SetInputModeUIOnly (Game|GetPlayerController 0) _output_get "DoNotLock")
  (UserInterface|Viewport|AddtoViewport _output_get 0)
  (Game|SetGamePaused true))

(event EventBeginPlay
  ;[1 1 1] start
  (Variables|/Script/Engine.PlayerController|SetbShowMouseCursor (Game|GetPlayerController 0) true)
  (Utilities|FlowControl|Sequence
    (:then_0
      (bind _returnvalue (UserInterface|CreateWidget "/Game/blueprints/start.start_C"))
      (bind _output_get (Variables|Default|Setstartmenu _returnvalue))
      (Input|SetInputModeUIOnly (Game|GetPlayerController 0) _output_get "DoNotLock")
      (UserInterface|Viewport|AddtoViewport _output_get 0)
      (Game|SetGamePaused true))
    (:then_1
      (bind _returnvalue_2 (UserInterface|CreateWidget "/Game/blueprints/basecharacterhealth.basecharacterhealth_C"))
      (bind _output_get_2 (Variables|Default|Sethealth _returnvalue_2))
      (UserInterface|Viewport|AddtoViewport _output_get_2 0))))

(fn ConstructionScript)