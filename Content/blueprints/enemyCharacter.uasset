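; Enemy character Blueprint that damages the player's base character on contact and awards score when killed.
; Overlapping a MybaseCharacter starts a looping timer that applies Damage at a DamagePerSecond rate, cleared when that overlap ends.
; On death, AffectHealth disables Pawn and WorldDynamic collision, adds score through the game mode, detaches the controller and destroys the actor after a delay.
; The construction script tints the mesh via a dynamic material using Bodycolor.
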(event Custom|damagethebasecharacter
  (Default|AffectHealth (Variables|Default|Getbasecharacter) (Variables|Default|Getdamage)))

(event EventBeginPlay)

(event Collision|EventActorBeginOverlap
  (params (OtherActor :type Actor%20Object%20Reference))
  (bind _asmybase_character (Utilities|Casting|CastToMybaseCharacter OtherActor))
  (Variables|Default|Setbasecharacter _asmybase_character)
  (Utilities|Time|SetTimerbyFunctionName 0 "damagethebasecharacter" (/ 1.0 (Variables|Default|Getdamage%20per%20second)) true))

(event EventTick
  (params (DeltaSeconds :type Float%20%28single-precision%29)))

(event EventAffectHealth
  (params (delta :type Float%20%28single-precision%29))
  (bind _capsulecomponent (Variables|Default|GetCapsuleComponent))
  (Class|BaseCharacter|CalculateHealth delta)
  (if (Variables|Default|GetisDead)
    (Collision|SetCollisionResponsetoChannel _capsulecomponent "ECC_WorldDynamic" "ECR_Ignore")
    (Collision|SetCollisionResponsetoChannel _capsulecomponent "ECC_Pawn" "ECR_Ignore")
    (bind _asmode (Utilities|Casting|CastTomode (Game|GetGameMode)))
    (Default|IncreaseScore _asmode 20)
    (Class|Pawn|DetachfromControllerPendingDestroy)
    (Utilities|FlowControl|Delay 3.0)
    (Actor|DestroyActor)))

(event Collision|EventActorEndOverlap
  (params (OtherActor :type Actor%20Object%20Reference))
  (if (== OtherActor (Variables|Default|Getbasecharacter))
    (Utilities|Time|ClearTimerbyFunctionName 0 "damagethebasecharacter")))

(fn ConstructionScript
  (bind _returnvalue (Rendering|Material|CreateDynamicMaterialInstance (Variables|Character|GetMesh) 0 0 :!class /Script/Engine.PrimitiveComponent))
  (bind _output_get (Variables|Default|Setdyna%20mat _returnvalue))
  (Rendering|Material|SetVectorParameterValue _output_get "bodycolor" (Variables|Default|Getbodycolor) :!class /Script/Engine.MaterialInstanceDynamic))