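; Game-mode-style Blueprint that runs enemy spawning, player respawn, scoring and an end-of-round scoreboard.
; BeginPlay starts a looping spawnenemy timer on the first Enemyspawn actor; respawn spawns and possesses a new character.
; Once the score reaches 100, Tick repeatedly rebuilds and saves the "savegame" scores, adding a scoreboard widget each frame.
; Only the placeholder entry insert (fixed name, zero score) is DoOnce-guarded; the Win screen is unconnected.
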(event Custom|respawn
  ;[1 1 1] respawn
  (bind _returnvalue (Game|SpawnActorfromClass "/Game/blueprints/MybaseCharacter.MybaseCharacter_C" (Variables|Default|Getplayer%20spawn%20transform) "Undefined" 0 0))
  (Pawn|Possess (Game|GetPlayerController 0) _returnvalue))

(event Custom|increase%20score
  (params (delta :type Integer))
  ;[1 1 1] increase score
  (bind _output_get (Variables|Default|Setsocre (+ delta (Variables|Default|Getsocre))))
  (Variables|Default|Setplayerscore (Utilities|Struct|Makeplayerscores "None" _output_get "0001.01.01-00.00.00")))

(event EventBeginPlay
  ;[1 1 1] spawn enemies
  (bind _outactors (Actor|GetAllActorsOfClass "/Game/blueprints/enemyspawn.enemyspawn_C"))
  (bind _output_get (Variables|Default|Setspawn (Utilities|Array|Get(acopy) _outactors)))
  (Utilities|Time|SetTimerbyFunctionName _output_get "spawnenemy" (/ 1.0 (Variables|Default|Getenemy)) true))

(event EventTick
  (params (DeltaSeconds :type Float%20%28single-precision%29))
  (bind _temp (Variables|Default|Gettemp))
  (if (>= (Variables|Default|Getsocre) 100)
    (Game|SetGamePaused false)
    (bind _returnvalue (SaveGame|LoadGamefromSlot "savegame"))
    (bind _assavegame (Utilities|Casting|CastTosavegame _returnvalue)
      (:then
        (for _array_element (Variables|/Game/blueprints/savegame.savegame_C|Getplayerscores _assavegame)
          (Utilities|FlowControl|Sequence
            (:then_0
              (if (<= (.score (Utilities|Struct|Breakplayerscores _array_element)) (Variables|Default|Getsocre))
                (Utilities|FlowControl|DoOnce false
                  (:Completed
                    (Utilities|Array|Add _temp (Utilities|Struct|Makeplayerscores "hujiaming" 0 "0001.01.01-00.00.00"))))))
            (:then_1
              (Utilities|Array|Add _temp _array_element))))
        (Utilities|FlowControl|Sequence
          (:then_0
            (Utilities|FlowControl|DoOnce false :!label _label
              (:Completed
                (Utilities|Array|Add _temp (Utilities|Struct|Makeplayerscores "hujiaming" 0 "0001.01.01-00.00.00")))))
          (:then_1
            (bind _returnvalue_2 (SaveGame|CreateSaveGameObject "/Game/blueprints/savegame.savegame_C" :!label _label_2))
            (bind _assavegame_2 (Utilities|Casting|CastTosavegame _returnvalue_2))
            (Variables|/Game/blueprints/savegame.savegame_C|Setplayerscores _assavegame_2 _temp)
            (SaveGame|SaveGametoSlot _returnvalue_2 "savegame")
            (bind _returnvalue_3 (UserInterface|CreateWidget "/Game/blueprints/scoreboard.scoreboard_C" 0 _temp))
            (UserInterface|Viewport|AddtoViewport _returnvalue_3 0))))
      (:CastFailed
        (Utilities|FlowControl|Sequence
          (:then_0
            (goto _label))
          (:then_1
            (goto _label_2)))))))

(fn ConstructionScript)