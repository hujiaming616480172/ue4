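; Game mode Blueprint that runs enemy spawning, player respawn, scoring and the win condition.
; BeginPlay starts a looping timer calling spawnenemy on the first Enemyspawn actor, at a rate set by Enemy.
; Respawn spawns and possesses a new MybaseCharacter at PlayerSpawnTransform.
; The increasescore event accumulates Socre, which Tick checks against 100 to pause the game and show the Win widget with mouse cursor.
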(event Custom|respawn
  ;[1 1 1] respawn
  (bind _returnvalue (Game|SpawnActorfromClass "/Game/blueprints/MybaseCharacter.MybaseCharacter_C" (Variables|Default|Getplayer%20spawn%20transform) "Undefined" 0 0))
  (Pawn|Possess (Game|GetPlayerController 0) _returnvalue))

(event Custom|increase%20score
  (params (delta :type Integer))
  ;[1 1 1] increase score
  (Variables|Default|Setsocre (+ delta (Variables|Default|Getsocre))))

(event EventBeginPlay
  ;[1 1 1] spawn enemies
  (bind _outactors (Actor|GetAllActorsOfClass "/Game/blueprints/enemyspawn.enemyspawn_C"))
  (bind _output_get (Variables|Default|Setspawn (Utilities|Array|Get(acopy) _outactors)))
  (Utilities|Time|SetTimerbyFunctionName _output_get "spawnenemy" (/ 1.0 (Variables|Default|Getenemy)) true))

(event EventTick
  (params (DeltaSeconds :type Float%20%28single-precision%29))
  (if (>= (Variables|Default|Getsocre) 100)
    (Game|SetGamePaused true)
    (bind _returnvalue (UserInterface|CreateWidget "/Game/blueprints/win.win_C"))
    (UserInterface|Viewport|AddtoViewport _returnvalue 0)
    (Variables|/Script/Engine.PlayerController|SetbShowMouseCursor (Game|GetPlayerController 0) true)))

(fn ConstructionScript)